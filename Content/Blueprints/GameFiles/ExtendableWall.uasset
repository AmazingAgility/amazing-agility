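; Extendable wall actor that builds a row of fence segments in the construction script, sized by an EndPoint vector.
; When EndPoint has a non-zero XY offset, its full length divided by a fixed segment spacing sets how many static mesh components are added.
; The base Wall gets FenceMesh, and each added component attaches to it, stepping along local X regardless of EndPoint's direction.
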(event EventBeginPlay)

(event Collision|EventActorBeginOverlap
  (params (OtherActor :type Actor%20Object%20Reference)))

(event EventTick
  (params (DeltaSeconds :type Float%20%28single-precision%29)))

(fn ConstructionScript
  (if (Math|Vector|NotEqual(Vector) (* (Variables|Default|GetEndPoint) "1.000000,1.000000,0.000000") "0, 0, 0" 0.0001)
    (for _index (range 1 (Math|Float|Floor (/ (Math|Vector|VectorLength (Variables|Default|GetEndPoint)) 152.0)))
      (Variables|Default|SetLastIndex _index)
      (Components|StaticMesh|SetStaticMesh (Variables|Default|GetWall) "/Game/Meshes/FenceMesh.FenceMesh")
      (bind _returnvalue (AddComponent|AddStaticMeshComponent true))
      (Transformation|AttachComponentToComponent _returnvalue (Variables|Default|GetWall) "None" "KeepWorld" "KeepWorld" "KeepRelative" true)
      (Transformation|SetRelativeLocationAndRotation _returnvalue (Math|Vector|MakeVector (* (Variables|Default|GetLastIndex) 152.0) 0.0 0.0) "0, 0, 0" false false))))