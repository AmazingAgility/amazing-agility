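; Checkpoint actor that registers as cleared when the wolf character passes through its trigger in the intended direction.
; On overlap end, it dots the wolf's velocity with the arrow component's forward vector, so only exits along the arrow count.
; A valid pass fires the CheckPointCleared dispatcher with the checkpoint number, hides the trigger and particles, and stops the trigger generating further overlaps.
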(event OnComponentEndOverlap(Trigger)
  (params (OverlappedComponent :type Primitive%20Component%20Object%20Reference) (OtherActor :type Actor%20Object%20Reference) (OtherComp :type Primitive%20Component%20Object%20Reference) (OtherBodyIndex :type Integer))
  (bind _trigger (Variables|Default|GetTrigger))
  ;[1 1 1] Checkpoint System -Cleared when overlapping ends
  (bind _aswolf_character (Utilities|Casting|CastToWolfCharacter OtherActor))
  (if (> (Math|Vector|DotProduct (Transformation|GetVelocity _aswolf_character) (Math|Rotator|GetRotationXVector (Transformation|GetWorldRotation (Variables|Default|GetArrow)))) 0.0)
    (Default|CallCheckPointCleared (Variables|Default|GetCheckPointNumber))
    (Development|SetHiddeninGame _trigger true true)
    (Variables|/Script/Engine.PrimitiveComponent|SetbGenerateOverlapEvents _trigger false)))

(fn ConstructionScript)